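; BP_TankCustomize is a tank actor whose turret and body meshes are chosen by TurretType and BodyType.
; The construction script switches on both values to set the TurretBase and BodyBase static meshes.
; SetTankTurret and SetTankBody repeat those switches for callers, with unmatched values falling back to the base meshes.
; Only SetTankTurret maps the third turret type to the MG turret; the construction script uses the base turret.
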(event EventBeginPlay)

(event Collision|EventActorBeginOverlap
  (params (OtherActor :type Actor%20Object%20Reference)))

(event EventTick
  (params (DeltaSeconds :type Float%20%28single-precision%29)))

(fn ConstructionScript
  (bind _turret_base (Variables|Default|GetTurret%20Base))
  (bind _body_base (Variables|Default|GetBody%20Base))
  (switch int (Math|Conversions|ToInteger(Byte) (Variables|Default|GetTurretType))
    (:Default
      (Components|StaticMesh|SetStaticMesh _turret_base "/Game/Assets/Meshes/SM_TankBaseTurret.SM_TankBaseTurret" :!label _label))
    (:0
      (goto _label))
    (:1
      (Components|StaticMesh|SetStaticMesh _turret_base "/Game/Assets/Meshes/SM_ATTankTurret.SM_ATTankTurret"))
    (:2
      (Components|StaticMesh|SetStaticMesh _turret_base "/Game/Assets/Meshes/SM_TankBaseTurret.SM_TankBaseTurret")))
  (switch int (Math|Conversions|ToInteger(Byte) (Variables|Default|GetBodyType))
    (:Default
      (Components|StaticMesh|SetStaticMesh _body_base "/Game/Assets/Meshes/SM_TankBase.SM_TankBase" :!label _label_2))
    (:0
      (goto _label_2))
    (:1
      (Components|StaticMesh|SetStaticMesh _body_base "/Game/Assets/Meshes/SM_TankArmored.SM_TankArmored"))))

(fn SetTankTurret
  (params (Turret%20Type :type Byte))
  (bind _turret_base (Variables|Default|GetTurret%20Base))
  (switch int (Math|Conversions|ToInteger(Byte) Turret%20Type)
    (:Default
      (Components|StaticMesh|SetStaticMesh _turret_base "/Game/Assets/Meshes/SM_TankBaseTurret.SM_TankBaseTurret" :!label _label))
    (:0
      (goto _label))
    (:1
      (Components|StaticMesh|SetStaticMesh _turret_base "/Game/Assets/Meshes/SM_ATTankTurret.SM_ATTankTurret"))
    (:2
      (Components|StaticMesh|SetStaticMesh _turret_base "/Game/Assets/Meshes/SM_MGPlayerTurret.SM_MGPlayerTurret"))))

(fn SetTankBody
  (params (Body%20Type :type Byte))
  (bind _body_base (Variables|Default|GetBody%20Base))
  (switch int (Math|Conversions|ToInteger(Byte) Body%20Type)
    (:Default
      (Components|StaticMesh|SetStaticMesh _body_base "/Game/Assets/Meshes/SM_TankBase.SM_TankBase" :!label _label))
    (:0
      (goto _label))
    (:1
      (Components|StaticMesh|SetStaticMesh _body_base "/Game/Assets/Meshes/SM_TankArmored.SM_TankArmored"))))