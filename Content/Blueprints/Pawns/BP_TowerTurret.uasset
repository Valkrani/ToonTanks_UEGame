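; Tower turret pawn Blueprint whose look is configured by its TowerType: standard, armored, MG or AT.
; The construction script switches on the type to set the turret and base meshes and position the projectile spawn point.
; The first three types share a base and muzzle position, while AT gets a heavy, lowered base and its own muzzle offset.
; The event graph holds no active logic.
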(event EventBeginPlay)

(event Collision|EventActorBeginOverlap
  (params (OtherActor :type Actor%20Object%20Reference)))

(event EventTick
  (params (DeltaSeconds :type Float%20%28single-precision%29)))

(fn ConstructionScript
  (bind _projectilespawnpoint (Variables|Default|GetProjectileSpawnPoint))
  (bind _turretmesh (Variables|Default|GetTurretMesh))
  (bind _basemesh (Variables|Default|GetBaseMesh))
  (switch int (Math|Conversions|ToInteger(Byte) (Variables|Default|GetTowerType))
    (:Default
      (Components|StaticMesh|SetStaticMesh _turretmesh "/Game/Assets/Meshes/SM_TowerTurret.SM_TowerTurret" :!label _label)
      (Components|StaticMesh|SetStaticMesh _basemesh "/Game/Assets/Meshes/SM_TowerBase.SM_TowerBase" :!label _label_2)
      (Transformation|SetRelativeLocation _projectilespawnpoint "90.000000,0.000000,95.000000" false false))
    (:0
      (goto _label))
    (:1
      (Components|StaticMesh|SetStaticMesh _turretmesh "/Game/Assets/Meshes/SM_TowerTurretArmored.SM_TowerTurretArmored")
      (goto _label_2))
    (:2
      (Components|StaticMesh|SetStaticMesh _turretmesh "/Game/Assets/Meshes/SM_MGTowerTurret.SM_MGTowerTurret")
      (goto _label_2))
    (:3
      (Components|StaticMesh|SetStaticMesh _turretmesh "/Game/Assets/Meshes/SM_TowerATTurret.SM_TowerATTurret")
      (Components|StaticMesh|SetStaticMesh _basemesh "/Game/Assets/Meshes/SM_TowerHeavyBase.SM_TowerHeavyBase")
      (Transformation|SetRelativeLocation _basemesh "0.000000,0.000000,-53.000000" false false)
      (Transformation|SetRelativeLocation _projectilespawnpoint "180.000000,0.000000,115.000000" false false))))