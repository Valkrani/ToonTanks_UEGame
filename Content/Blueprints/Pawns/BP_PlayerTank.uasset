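; Player tank pawn whose look is assembled from its TurretType and BodyType settings.
; LoadPlayerMeshes picks the turret mesh (base, anti-tank or MG) and hull mesh (base or armored), falling back to base for other values.
; It also moves the projectile spawn point farther forward for the anti-tank turret.
; The Construction Script and BeginPlay both run it, and BeginPlay also enables gravity on the capsule.
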(event EventBeginPlay
  (CallFunction|LoadPlayerMeshes)
  (Physics|SetEnableGravity (Variables|Default|GetCapsuleComp) true))

(event Collision|EventActorBeginOverlap
  (params (OtherActor :type Actor%20Object%20Reference)))

(event EventTick
  (params (DeltaSeconds :type Float%20%28single-precision%29)))

(fn ConstructionScript
  (CallFunction|LoadPlayerMeshes))

(fn LoadPlayerMeshes
  (bind _turretmesh (Variables|Default|GetTurretMesh))
  (bind _basemesh (Variables|Default|GetBaseMesh))
  (bind _projectilespawnpoint (Variables|Default|GetProjectileSpawnPoint))
  (switch int (Math|Conversions|ToInteger(Byte) (Variables|Default|GetTurretType))
    (:Default
      (Components|StaticMesh|SetStaticMesh _turretmesh "/Game/Assets/Meshes/SM_TankBaseTurret.SM_TankBaseTurret" :!label _label)
      (Transformation|SetRelativeLocation _projectilespawnpoint "100.000000,0.000000,85.000000" false false :!label _label_2))
    (:0
      (goto _label))
    (:1
      (Components|StaticMesh|SetStaticMesh _turretmesh "/Game/Assets/Meshes/SM_ATTankTurret.SM_ATTankTurret")
      (Transformation|SetRelativeLocation _projectilespawnpoint "170.000000,0.000000,85.000000" false false))
    (:2
      (Components|StaticMesh|SetStaticMesh _turretmesh "/Game/Assets/Meshes/SM_MGPlayerTurret.SM_MGPlayerTurret")
      (goto _label_2)))
  (switch int (Math|Conversions|ToInteger(Byte) (Variables|Default|GetBodyType))
    (:Default
      (Components|StaticMesh|SetStaticMesh _basemesh "/Game/Assets/Meshes/SM_TankBase.SM_TankBase" :!label _label_3))
    (:0
      (goto _label_3))
    (:1
      (Components|StaticMesh|SetStaticMesh _basemesh "/Game/Assets/Meshes/SM_TankArmored.SM_TankArmored"))))