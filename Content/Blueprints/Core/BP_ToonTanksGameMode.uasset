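; Game mode Blueprint for ToonTanks that handles the UI when a game starts and ends.
; StartGame either shows the mouse cursor and main menu, or shows the start-game widget and adds the player stats widget after a short delay.
; GameOver creates the game-over widget, passes it the win result and adds it to the viewport.
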(event EventStartGame
  (params (bIsMainMenu :type Boolean))
  (if bIsMainMenu
    (Variables|/Script/Engine.PlayerController|SetbShowMouseCursor (Game|GetPlayerController (Game|GetPlayerState 0)) true)
    (bind _returnvalue (UserInterface|CreateWidget "/Game/Blueprints/Widgets/WBP_MainMenu.WBP_MainMenu_C"))
    (UserInterface|Viewport|AddtoViewport _returnvalue 0)
    (else
      (bind _returnvalue_2 (UserInterface|CreateWidget "/Game/Blueprints/Widgets/WBP_StartGameWidget.WBP_StartGameWidget_C"))
      (UserInterface|Viewport|AddtoViewport _returnvalue_2 0)
      (Utilities|FlowControl|Delay 3.0)
      (bind _returnvalue_3 (UserInterface|CreateWidget "/Game/Blueprints/Widgets/WBP_PlayerStats.WBP_PlayerStats_C" (Game|GetPlayerController 0)))
      (UserInterface|Viewport|AddtoViewport _returnvalue_3 0))))

(event EventGameOver
  (params (bWonGame :type Boolean))
  (bind _returnvalue (UserInterface|CreateWidget "/Game/Blueprints/Widgets/WBP_GameOverWidget.WBP_GameOverWidget_C"))
  (Variables|/Game/Blueprints/Widgets/WBP_GameOverWidget.WBP_GameOverWidget_C|SetGameWon _returnvalue bWonGame)
  (UserInterface|Viewport|AddtoViewport _returnvalue 0))

(fn ConstructionScript)