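; Health pickup actor that gives health to a player tank on overlap, then respawns after a cooldown.
; Its mesh spins by a fixed step each Tick, independent of delta time.
; Sphere overlap with BP_PlayerTank calls PickupHealth, hides the mesh and sets a cooldown flag that blocks further pickups.
; A ten-second timer calls ResetCooldown to clear the flag and show the mesh again.
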(event OnComponentBeginOverlap(Sphere)
  (params (OverlappedComponent :type Primitive%20Component%20Object%20Reference) (OtherActor :type Actor%20Object%20Reference) (OtherComp :type Primitive%20Component%20Object%20Reference) (OtherBodyIndex :type Integer) (bFromSweep :type Boolean) (SweepResult :type Hit%20Result%20Structure%20%28by%20ref%29))
  (if (not (Variables|Default|GetIsOnCooldown))
    (bind _asbp_player_tank (Utilities|Casting|CastToBP_PlayerTank OtherActor))
    (Default|PickupHealth _asbp_player_tank)
    (Rendering|SetVisibility (Variables|Default|GetSM_TankBase) false false)
    (Variables|Default|SetIsOnCooldown true)
    (Utilities|Time|SetTimerbyFunctionName 0 "ResetCooldown" 1e+01)))

(event EventBeginPlay)

(event Collision|EventActorBeginOverlap
  (params (OtherActor :type Actor%20Object%20Reference)))

(event EventTick
  (params (DeltaSeconds :type Float%20%28single-precision%29))
  (Transformation|AddLocalRotation (Variables|Default|GetSM_TankBase) "0.000000,0.500000,0.000000" false false))

(fn ConstructionScript)

(fn ResetCooldown
  (Variables|Default|SetIsOnCooldown false)
  (Rendering|SetVisibility (Variables|Default|GetSM_TankBase) true false))